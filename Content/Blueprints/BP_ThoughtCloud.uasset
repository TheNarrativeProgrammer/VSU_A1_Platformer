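; BP_ThoughtCloud is a moving cloud actor that reacts to overlaps and breaks apart when the third-person character touches it.
; A timeline moves its mesh from the relative origin toward FinalLocation.
; Capsule overlap sends CanTakeDamageMessage to any overlapping actor.
; For the character only, it also spawns dust, swaps the regular flipbook for the destroy flipbook, and destroys itself after a short delay.
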(event `self.ReceiveBeginPlay`
  (bind _paperflipbook_destroy (`self.PaperFlipbook_Destroy`))
  ;[1 1 1] Move cloud
  (`PaperFlipbookComponent.Stop` _paperflipbook_destroy)
  (`SceneComponent.SetVisibility` _paperflipbook_destroy false false)
  (`SceneComponent.SetVisibility` (`self.PaperFlipbook_Regular`) true false)
  (bind (_direction _alpha) (`Timeline|CloudMovementTimeline`)
    (:`Update`
      (`SceneComponent.K2_SetRelativeLocation` (`self.sm_ThoughtCloud`) (`KismetMathLibrary.VLerp` (0.0 0.0 0.0) (`self._finalLocation`) _alpha) false false))))

(event `self.Capsule.OnComponentBeginOverlap`
  (params (OverlappedComponent :type "PrimitiveComponent Object Reference") (OtherActor :type "Actor Object Reference") (OtherComp :type "PrimitiveComponent Object Reference") (OtherBodyIndex :type Integer) (bFromSweep :type Boolean) (SweepResult :type "HitResult Structure (by ref)"))
  (bind _paperflipbook_destroy (`self.PaperFlipbook_Destroy`))
  (message `/Game/Blueprints/Interfaces/BPI_CanTakeDamage.CanTakeDamage` OtherActor)
  (cast `/Game/ThirdPerson/Blueprints/BP_ThirdPersonCharacter` OtherActor)
  (`GameplayStatics.SpawnEmitterAtLocation` "/Game/StarterContent/Particles/P_Ambient_Dust.P_Ambient_Dust" (`SceneComponent.K2_GetComponentLocation` (`self.sm_ThoughtCloud`)))
  (`SceneComponent.SetVisibility` (`self.PaperFlipbook_Regular`) false false)
  (`PaperFlipbookComponent.PlayFromStart` _paperflipbook_destroy)
  (`SceneComponent.SetVisibility` _paperflipbook_destroy true false)
  (`KismetSystemLibrary.Delay` 0.8)
  (`self.K2_DestroyActor`))

(fn `UserConstructionScript`)