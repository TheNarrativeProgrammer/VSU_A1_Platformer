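; BP_CalMeeting is a calendar meeting pickup that triggers the player's win state when collected.
; Overlap by BP_ThirdPersonCharacter disables the box collision and runs a one-time timeline.
; The timeline lerps the actor between its start location and the player's live position with a Z offset, producing a lift-and-home motion.
; When it finishes, OnPickUp destroys the actor, then WinState is called on the character.
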(event `self.Box.OnComponentBeginOverlap`
  (params (OverlappedComponent :type "PrimitiveComponent Object Reference") (OtherActor :type "Actor Object Reference") (OtherComp :type "PrimitiveComponent Object Reference") (OtherBodyIndex :type Integer) (bFromSweep :type Boolean) (SweepResult :type "HitResult Structure (by ref)"))
  ;[1 1 1] Move BP up and towards player on collision
  ;
  ; On overlap, check if overlapping actor is BP_character and get ref. Lerp from this BP's current location to the player location while adding to z-axis to make BP move up.
  (bind _asbp_third_person_character (cast `/Game/ThirdPerson/Blueprints/BP_ThirdPersonCharacter` OtherActor))
  (`PrimitiveComponent.SetCollisionEnabled` (`self.Box`) "NoCollision")
  (`/Engine/EditorBlueprintResources/StandardMacros.DoOnce` false
    (:`Completed`
      (set `self.StartLocation` (`self.K2_GetActorLocation`))
      (bind (_direction _zoffset _alpha) (`Timeline|CalMettingPickuP`)
        (:`Update`
          (`self.K2_SetActorLocation` (`KismetMathLibrary.VLerp` (+ (`self.K2_GetActorLocation` OtherActor) (`KismetMathLibrary.MakeVector` 0.0 0.0 _zoffset)) (`self.StartLocation`) _alpha)))
        (:`Finished`
          (`self.OnPickUp`)
          (`/Game/ThirdPerson/Blueprints/BP_ThirdPersonCharacter.WinState` _asbp_third_person_character))))))

(fn `OnPickUp`
  ;[1 1 1] Destroy on pickup
  (`self.K2_DestroyActor`))

(fn `UserConstructionScript`)