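; Calendar actor that displays eleven hourly timeslot meshes from 8am to 6pm and schedules two random meetings on BeginPlay.
; It draws two unique keys from Keys, sets a material on the matching slot meshes, then spawns BP_CalMeeting at each key's preset location.
; The last two slots share a spawn location, and the keys clear after a short delay.
; Tick offsets the calendar on Y from the player's follow camera.
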(event `self.ReceiveBeginPlay`
  (bind _uniquekeys (`self.UniqueKeys`))
  (bind _output (`|GetArrayItem` (`self.UniqueKeys`) 1))
  ;[1 1 1] Set up Calendar look and meeting times. Generate spawn of meetings
  ;;[0.09255 0.2702 1] Set up Arrays
  ;; - CalendarTimeSlots: array of static meshes that are blue by default. These represent timeslots on a calendar
  ;; - NOTE: Keys array is set up outside a BP. It constist of 11 elements
  ;; - UniqueKeys: array of 2 randomly selected elements from Keys array. This represents 2 meetings randomly selected from the 11 possible times.
  (`KismetArrayLibrary.Array_Clear` (`self.UniqueKeys`)) ; Clear keys. WIll be use later when \ndifferent levels are implemented
  (bind _asbp_third_person_character (cast `/Game/Blueprints/VSU/BP/BP_ThirdPersonCharacter` (`GameplayStatics.GetPlayerCharacter` 0))) ; Get Reference to player
  (set `self.BP Third Person Character` _asbp_third_person_character)
  (set `self.CalendarTimeSlots` (`|MakeArray` (`self.8:00am`) (`self.9:00am`) (`self.10:00am`) (`self.11:00am`) (`self.12:00pm`) (`self.1:00pm`) (`self.2:00pm`) (`self.3:00pm`) (`self.4:00pm`) (`self.5:00pm`) (`self.6:00pm`))) ; Save array to variable
  (while (< (`KismetArrayLibrary.Array_Length` _uniquekeys) 2)
    (`KismetArrayLibrary.Array_AddUnique` _uniquekeys (`KismetArrayLibrary.Array_Random` (`self.Keys`))))
  (`|ExecutionSequence`
    (:`then_0`
      ;;[0.09255 0.2702 1] Change material of element 0 and element 1 in Uniquekeys array. This indicates that a meeting is at this time on the calendar
      (`PrimitiveComponent.SetMaterial` (`|GetArrayItem` (`self.CalendarTimeSlots`) (`|GetArrayItem` (`self.UniqueKeys`))) 0 "/DatasmithContent/Materials/AliasReference.AliasReference")
      (`PrimitiveComponent.SetMaterial` (`|GetArrayItem` (`self.CalendarTimeSlots`) _output) _output "/DatasmithContent/Materials/AliasReference.AliasReference"))
    (:`then_1`
      ;;[0.09255 0.2702 1] Set location of Element 0 and spawn BP at location
      (switch `int` (`|GetArrayItem` (`self.UniqueKeys`))
        (:`0`
          (set `self.CalendarTaskSpawnA` (`self.CalendarTaskLocation0`)))
        (:`1`
          (set `self.CalendarTaskSpawnA` (`self.CalendarTaskLocation1`)))
        (:`2`
          (set `self.CalendarTaskSpawnA` (`self.CalendarTaskLocation2`)))
        (:`3`
          (set `self.CalendarTaskSpawnA` (`self.CalendarTaskLocation3`)))
        (:`4`
          (set `self.CalendarTaskSpawnA` (`self.CalendarTaskLocation4`)))
        (:`5`
          (set `self.CalendarTaskSpawnA` (`self.CalendarTaskLocation5`)))
        (:`6`
          (set `self.CalendarTaskSpawnA` (`self.CalendarTaskLocation6`)))
        (:`7`
          (set `self.CalendarTaskSpawnA` (`self.CalendarTaskLocation7`)))
        (:`8`
          (set `self.CalendarTaskSpawnA` (`self.CalendarTaskLocation8`)))
        (:`9`
          (set `self.CalendarTaskSpawnA` (`self.CalendarTaskLocation9`)))
        (:`10`
          (set `self.CalendarTaskSpawnA` (`self.CalendarTaskLocation9`))))
      (`|SpawnActorFromClass` "/Game/Blueprints/VSU/BP/Calendar/BP_CalMeeting.BP_CalMeeting_C" (`KismetMathLibrary.Conv_VectorToTransform` (`self.CalendarTaskSpawnA`)) "Undefined" "MultiplyWithRoot" null null))
    (:`then_2`
      ;;[0.09255 0.2702 1] Set location of Element 1 and spawn BP at location
      (switch `int` (`|GetArrayItem` (`self.UniqueKeys`) 1)
        (:`0`
          (set `self.CalendarTaskSpawnA` (`self.CalendarTaskLocation0`)))
        (:`1`
          (set `self.CalendarTaskSpawnA` (`self.CalendarTaskLocation1`)))
        (:`2`
          (set `self.CalendarTaskSpawnA` (`self.CalendarTaskLocation2`)))
        (:`3`
          (set `self.CalendarTaskSpawnA` (`self.CalendarTaskLocation3`)))
        (:`4`
          (set `self.CalendarTaskSpawnA` (`self.CalendarTaskLocation4`)))
        (:`5`
          (set `self.CalendarTaskSpawnA` (`self.CalendarTaskLocation5`)))
        (:`6`
          (set `self.CalendarTaskSpawnA` (`self.CalendarTaskLocation6`)))
        (:`7`
          (set `self.CalendarTaskSpawnA` (`self.CalendarTaskLocation7`)))
        (:`8`
          (set `self.CalendarTaskSpawnA` (`self.CalendarTaskLocation8`)))
        (:`9`
          (set `self.CalendarTaskSpawnA` (`self.CalendarTaskLocation9`)))
        (:`10`
          (set `self.CalendarTaskSpawnA` (`self.CalendarTaskLocation9`))))
      (`|SpawnActorFromClass` "/Game/Blueprints/VSU/BP/Calendar/BP_CalMeeting.BP_CalMeeting_C" (`KismetMathLibrary.Conv_VectorToTransform` (`self.CalendarTaskSpawnA`)) "Undefined" "MultiplyWithRoot" null null))
    (:`then_3`
      ;;[0.09255 0.2702 1] Clear keys
      (`KismetSystemLibrary.Delay` 0.2)
      (`KismetArrayLibrary.Array_Clear` (`self.UniqueKeys`)))))

(event `self.ReceiveTick`
  (params (DeltaSeconds :type "Float (single-precision)"))
  (bind _defaultsceneroot (`self.DefaultSceneRoot`))
  (bind (_returnvalue_x _returnvalue_y _returnvalue_z) (`KismetMathLibrary.BreakVector` (`SceneComponent.K2_GetComponentLocation` _defaultsceneroot)))
  (bind (_returnvalue_x_2 _returnvalue_y_2) (`KismetMathLibrary.BreakVector` (`SceneComponent.K2_GetComponentLocation` (`/Game/Blueprints/VSU/BP/BP_ThirdPersonCharacter.FollowCamera` (`self.BP Third Person Character`)))))
  ;[1 1 1] Update Location on y-axis based on Camera position
  ;
  ; This moves the Calender based on the players lateral movement
  (if (and (`KismetSystemLibrary.IsValid` (`self.BP Third Person Character`)) (`KismetSystemLibrary.IsValid` (`self.DefaultSceneRoot`)))
    (`SceneComponent.K2_SetWorldTransform` _defaultsceneroot (`KismetMathLibrary.MakeTransform` (`KismetMathLibrary.MakeVector` _returnvalue_x (- _returnvalue_y_2 800.0) _returnvalue_z)) false false)))

(fn `UserConstructionScript`)