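; BP_CloudSpawner is an actor that spawns BP_ThoughtCloud actors at its own location.
; A timeline started on BeginPlay sets the spawn frequency through its Fire Cloud event track.
; MoveCloudSpawn_Event, noted as called from MoveCloudSpawner, moves the spawner to the height of the player character's mesh while keeping its X and Y, so later clouds appear at that height.
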(event `self.ReceiveBeginPlay`
  ;[1 1 1] Frequency Clouds are spawned at
  (`Timeline|SpawnCloudTimeline`
    (:`FireCloud`
      (`|SpawnActorFromClass` "/Game/Blueprints/VSU/BP/Clouds/BP_ThoughtCloud.BP_ThoughtCloud_C" (`KismetMathLibrary.Conv_VectorToTransform` (`self.K2_GetActorLocation`)) "Undefined" "MultiplyWithRoot" null null))))

(event `MoveCloudSpawn_Event`
  (params (vecto :type "Vector Structure"))
  (bind _defaultsceneroot (`self.DefaultSceneRoot`))
  (bind (_returnvalue_x _returnvalue_y) (`KismetMathLibrary.BreakVector` (`SceneComponent.K2_GetComponentLocation` _defaultsceneroot)))
  (bind (_returnvalue_x_2 _returnvalue_y_2 _returnvalue_z) (`KismetMathLibrary.BreakVector` (`SceneComponent.K2_GetComponentLocation` (`Character.Mesh` (`GameplayStatics.GetPlayerCharacter` 0)))))
  ;[1 0.04978 0] Called in MoveCloudSpawner. This moves this BP, the CloudSpawner to a new location on Z-axis
  (`SceneComponent.K2_SetWorldTransform` _defaultsceneroot (`KismetMathLibrary.MakeTransform` (`KismetMathLibrary.MakeVector` _returnvalue_x _returnvalue_y _returnvalue_z)) false false))

(fn `UserConstructionScript`)