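; BP_ThoughtCloud is a moving cloud hazard that travels from a start to a final location and sends a damage interface message to actors overlapping its capsule.
; A timeline lerps the cloud's relative location from BeginPlay.
; Player overlap spawns a dust emitter, then shares the end-of-track exit: swap the regular flipbook for the destroy flipbook, wait briefly, and destroy the actor.
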(event `self.ReceiveBeginPlay`
  (bind _paperflipbook_destroy (`self.PaperFlipbook_Destroy`))
  ;[1 1 1] On Spawn, move cloud from start location to finished
  (`PaperFlipbookComponent.Stop` _paperflipbook_destroy)
  (`SceneComponent.SetVisibility` _paperflipbook_destroy false false)
  (`SceneComponent.SetVisibility` (`self.PaperFlipbook_Regular`) true false)
  (bind (_direction _alpha) (`Timeline|CloudMovementTimeline` :!via `PlayFromStart`)
    (:`Update`
      (`SceneComponent.K2_SetRelativeLocation` (`self.sm_ThoughtCloud`) (`KismetMathLibrary.VLerp` (`self.start`) (`self._finalLocation`) _alpha) false false))
    (:`Finished`
      (`self.DestroyCloudAtEnd`) ; If player doesn't collide with cloud, destroy is at end of track
    )))

(event `self.Capsule.OnComponentBeginOverlap`
  (params (OverlappedComponent :type "PrimitiveComponent Object Reference") (OtherActor :type "Actor Object Reference") (OtherComp :type "PrimitiveComponent Object Reference") (OtherBodyIndex :type Integer) (bFromSweep :type Boolean) (SweepResult :type "HitResult Structure (by ref)"))
  (bind _paperflipbook_destroy (`self.PaperFlipbook_Destroy`))
  ;[1 1 1] On Overlap, check if the object has "CanTakeDamage" interface and call event.
  ;
  ; Toggle visiblity of standard sprite flipbook - OFF
  ; Toggle visiblity of destrory sprite flipbook - ON
  (message `/Game/Blueprints/VSU/BP/Interfaces/BPI_CanTakeDamage.CanTakeDamage` OtherActor 0)
  (cast `/Game/Blueprints/VSU/BP/BP_ThirdPersonCharacter` OtherActor)
  (`GameplayStatics.SpawnEmitterAtLocation` "/Game/StarterContent/Particles/P_Ambient_Dust.P_Ambient_Dust" (`SceneComponent.K2_GetComponentLocation` (`self.sm_ThoughtCloud`)))
  (`SceneComponent.SetVisibility` (`self.PaperFlipbook_Regular`) false false :!label _label)
  (`PaperFlipbookComponent.PlayFromStart` _paperflipbook_destroy)
  (`SceneComponent.SetVisibility` _paperflipbook_destroy true false)
  (`KismetSystemLibrary.Delay` 0.8)
  (`self.K2_DestroyActor`))

(event `DestroyCloudAtEnd`
  ;[1 1 1] On Overlap, check if the object has "CanTakeDamage" interface and call event.
  ;
  ; Toggle visiblity of standard sprite flipbook - OFF
  ; Toggle visiblity of destrory sprite flipbook - ON
  (goto _label))

(fn `UserConstructionScript`)