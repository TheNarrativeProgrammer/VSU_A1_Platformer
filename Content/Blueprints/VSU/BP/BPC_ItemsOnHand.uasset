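; Component that toggles the visibility state of items on hand: cards, wallet and fob.
; Each item has paired On and Off functions that set a boolean flag and broadcast it through that item's SetVisibility event dispatcher.
; The component changes no visuals here, leaving that to whatever binds to the dispatchers.
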(fn `AdjustVisibilityCardsOff`
  (locals (isVisibileCards :type Boolean) (isVisibileWallet :type Boolean) (isVisibileWalletFob :type Boolean))
  (bind _output_get (set `local.isVisibileCards` false))
  (`self.SetVisibilityCard` _output_get))

(fn `AdjustVisibilityCardsOn`
  (locals (isVisibileCards :type Boolean) (isVisibileWallet :type Boolean) (isVisibileWalletFob :type Boolean))
  (bind _output_get (set `local.isVisibileCards` true))
  (`self.SetVisibilityCard` _output_get))

(fn `AdjustVisibilityFobOff`
  (locals (isVisibileCards :type Boolean) (isVisibileWallet :type Boolean) (isVisibileWalletFob :type Boolean))
  (bind _output_get (set `local.isVisibileWalletFob` false))
  (`self.SetVisibilityFob` _output_get))

(fn `AdjustVisibilityFobOn`
  (locals (isVisibileCards :type Boolean) (isVisibileWallet :type Boolean) (isVisibileWalletFob :type Boolean))
  (bind _output_get (set `local.isVisibileWalletFob` true))
  (`self.SetVisibilityFob` _output_get))

(fn `AdjustVisibilityWalletOff`
  (locals (isVisibileCards :type Boolean) (isVisibileWallet :type Boolean) (isVisibileWalletFob :type Boolean))
  (bind _output_get (set `local.isVisibileWallet` false))
  (`self.SetVisibilityWallet` _output_get))

(fn `AdjustVisibilityWalletOn`
  (locals (isVisibileCards :type Boolean) (isVisibileWallet :type Boolean) (isVisibileWalletFob :type Boolean))
  (bind _output_get (set `local.isVisibileWallet` true))
  (`self.SetVisibilityWallet` _output_get))