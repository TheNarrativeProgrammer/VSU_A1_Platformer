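; BP_CalendarEvent is a calendar-event pickup that flies to the player on contact, then destroys itself.
; A box overlap with BP_ThirdPersonCharacter disables the box's collision and saves the actor's start location.
; A one-shot timeline lerps the actor toward the player's live position plus an animated Z offset, matching the player's scale.
; OnPickUp runs when the timeline finishes and only destroys the actor, while DropItem is an empty stub.
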(event `self.ReceiveBeginPlay`)

(event `Drop Item`)

(event `self.Box.OnComponentBeginOverlap`
  (params (OverlappedComponent :type "PrimitiveComponent Object Reference") (OtherActor :type "Actor Object Reference") (OtherComp :type "PrimitiveComponent Object Reference") (OtherBodyIndex :type Integer) (bFromSweep :type Boolean) (SweepResult :type "HitResult Structure (by ref)"))
  (bind _asbp_third_person_character (cast `/Game/ThirdPerson/Blueprints/BP_ThirdPersonCharacter` OtherActor))
  (set `self.As BP Third Person Character` _asbp_third_person_character)
  (`PrimitiveComponent.SetCollisionEnabled` (`self.Box`) "NoCollision") ; Turn off collision once player collides and cast succeeds. \nThis prevents errrors from a CloudBP failing the cast and making\nNULL reference for blue line (ref)
  (`/Engine/EditorBlueprintResources/StandardMacros.DoOnce` false
    (:`Completed`
      (set `self.Start Location` (`self.K2_GetActorLocation`)) ; Save current location of this Actor.\nUse as starting location for Lerp
      (bind (_direction _zoffset _alpha) (`Timeline|PickUpTimeline`)
        (:`Update`
          (`self.K2_SetActorLocation` (`KismetMathLibrary.VLerp` (`self.Start Location`) (+ (`self.K2_GetActorLocation` OtherActor) (`KismetMathLibrary.MakeVector` 0.0 0.0 _zoffset)) _alpha))
          (`self.SetActorScale3D` (`self.GetActorScale3D` OtherActor)))
        (:`Finished`
          (`self.OnPickUp` _asbp_third_person_character))))))

(fn `OnPickUp`
  (params (Player :type "/Game/ThirdPerson/Blueprints/BP_ThirdPersonCharacter Object Reference"))
  (`self.K2_DestroyActor`))

(fn `UserConstructionScript`)