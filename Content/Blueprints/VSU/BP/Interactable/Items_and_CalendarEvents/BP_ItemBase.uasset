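; Base actor for pickup items that bounce toward the player and are collected on touch.
; Box overlap with BP_ThirdPersonCharacter disables collision, then a timeline lerps the item from its start location to the player's live position with an added Z offset.
; When the timeline finishes, OnPickUp passes ItemIndex to the character's PickUpItem, plays a sound at the world origin and destroys the actor.
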(event `self.Box.OnComponentBeginOverlap`
  (params (OverlappedComponent :type "PrimitiveComponent Object Reference") (OtherActor :type "Actor Object Reference") (OtherComp :type "PrimitiveComponent Object Reference") (OtherBodyIndex :type Integer) (bFromSweep :type Boolean) (SweepResult :type "HitResult Structure (by ref)"))
  ;[1 1 1] Animation for picking up an item. Lerps from item location to player location while adding upward movement to make the item bounce up.
  ;
  ; Calls Onpickup function.
  (bind _asbp_third_person_character (cast `/Game/Blueprints/VSU/BP/BP_ThirdPersonCharacter` OtherActor))
  (set `self.As BP Third Person Character` _asbp_third_person_character)
  (`PrimitiveComponent.SetCollisionEnabled` (`self.Box`) "NoCollision") ; Turn off collision once player collides and cast succeeds. \nThis prevents errrors from a CloudBP failing the cast and making\nNULL reference for blue line (ref)
  (`/Engine/EditorBlueprintResources/StandardMacros.DoOnce` false
    (:`Completed`
      (set `self.Start Location` (`self.K2_GetActorLocation`)) ; Save current location of this Actor.\nUse as starting location for Lerp
      (bind (_direction _zoffset _alpha) (`Timeline|PickUpTimeline`)
        (:`Update`
          (`self.K2_SetActorLocation` (`KismetMathLibrary.VLerp` (`self.Start Location`) (+ (`self.K2_GetActorLocation` OtherActor) (`KismetMathLibrary.MakeVector` 0.0 0.0 _zoffset)) _alpha)))
        (:`Finished`
          (`self.OnPickUp` _asbp_third_person_character))))))

(fn `OnPickUp`
  (params (Player :type "/Game/Blueprints/VSU/BP/BP_ThirdPersonCharacter Object Reference"))
  ;[1 1 1] Destry actor and send message to BP_Character.
  ;
  ; Message to BP_Character updates the Item-array so that when a dropped item (which is removed from the rray on drop) is picked up by the player, the item is added back into the array.
  (`/Game/Blueprints/VSU/BP/BP_ThirdPersonCharacter.PickUpItem` (`self.As BP Third Person Character`) (`self.Item Index`))
  (`GameplayStatics.SpawnSoundAtLocation` "/Game/Blueprints/VSU/Sounds/zapsplat_foley_piggy_bank_ceramic_banknote_insert_stuff_in_001_73467.zapsplat_foley_piggy_bank_ceramic_banknote_insert_stuff_in_001_73467" (0.0 0.0 0.0) (struct) 1.0 1.0 0.0 null null)
  (`self.K2_DestroyActor`))

(fn `UserConstructionScript`)