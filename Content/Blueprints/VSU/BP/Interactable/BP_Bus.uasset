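; BP_Bus is an interactable bus whose cube mesh moves between start and end locations on a timeline that plays from BeginPlay.
; Player overlap stops the timeline and shows an interact prompt, while leaving resumes it and hides prompts.
; OnInteract restarts the bus if the player's ItemsOnHand contains item 0 or Testing is set, otherwise showing a missing-item prompt.
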(event `StartBus`
  ;[1 1 1] Start and stop bus based on the flowing:
  ; If player is overlapping collision box - stop
  ; If player has Item-Card and pressed E
  (bind (_direction _alpha) (`Timeline|BusTravelTimeline` :!label _label)
    (:`Update`
      (`SceneComponent.K2_SetRelativeLocation` (`self.Cube`) (`KismetMathLibrary.VLerp` (`self.Start Location`) (`self.End Location`) _alpha) false false)
      (if false
        _))))

(event `self.ReceiveBeginPlay`
  ;[1 1 1] Start and stop bus based on the flowing:
  ; If player is overlapping collision box - stop
  ; If player has Item-Card and pressed E
  (goto _label))

(event `StopBus`
  ;[1 1 1] Start and stop bus based on the flowing:
  ; If player is overlapping collision box - stop
  ; If player has Item-Card and pressed E
  (goto _label :!via `Stop`))

(event `self.ReceiveActorBeginOverlap`
  (params (OtherActor :type "Actor Object Reference"))
  ;[1 1 1] Start bus & toggle message - when player triggers overlap
  ; Stop  bus & toggle message - when player Ends overlap
  (cast `/Game/Blueprints/VSU/BP/BP_ThirdPersonCharacter` OtherActor)
  (set `self.IsOverLap` true)
  (`self.StopBus`)
  (`SceneComponent.SetVisibility` (`self.Interact Prompt`) true false))

(event `self.ReceiveActorEndOverlap`
  (params (OtherActor :type "Actor Object Reference"))
  ;[1 1 1] Start bus & toggle message - when player triggers overlap
  ; Stop  bus & toggle message - when player Ends overlap
  (cast `/Game/Blueprints/VSU/BP/BP_ThirdPersonCharacter` OtherActor)
  (set `self.IsOverLap` false)
  (`self.StartBus`)
  (`SceneComponent.SetVisibility` (`self.Interact Prompt`) false false)
  (`SceneComponent.SetVisibility` (`self.Missing Item Prompt`) false false))

(event `/Game/Blueprints/VSU/BP/Interfaces/BPI_Interactable.OnInteract`
  (params (Player :type "/Game/Blueprints/VSU/BP/BP_ThirdPersonCharacter Object Reference"))
  ;[1 1 1] When player presses E, this object has interface that listens for message. OnkeyPress, this checks if player has the item-card, which is index =1, and if they have that item, the bus starts back up.
  (if (`self.testing`)
    _
    (else
      _))
  (if (or (!= (`KismetArrayLibrary.Array_Find` (`/Game/Blueprints/VSU/BP/BP_ThirdPersonCharacter.ItemsOnHand` Player)) -1) (`self.testing`))
    (`self.StartBus`)
    (else
      (`SceneComponent.SetVisibility` (`self.Missing Item Prompt`) true false))))

(fn `UserConstructionScript`)